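; Player controller for a first-person character that chops destroyables with an axe and can throw it.
; Each tick a camera line trace selects the aimed destroyable, shows its damage UI and pauses its healing.
; Attack plays a level-sequence swing, applies damage after a short delay and repeats while held.
; Special attack hides the held axe and spawns a projectile aimed at a target actor placed on the trace impact.
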(event EventBeginPlay
  (bind _fpc (CallFunction|GetFPC))
  (bind _output_get (Variables|Default|SetFPC _fpc))
  (Rendering|SetVisibility (Variables|/Game/FirstPersonBP/Blueprints/FirstPersonCharacter.FirstPersonCharacter_C|GetAxe _output_get) false false)
  (bind _returnvalue (UserInterface|CreateWidget "/Game/EthanBluePrints/WBP_PlayerUI.WBP_PlayerUI_C" self))
  (bind _output_get_2 (Variables|Default|SetMyUI _returnvalue))
  (UserInterface|Viewport|AddtoViewport _output_get_2 0)
  (Default|SetVisibilityDamagesOfDestroyable (Variables|Default|GetMyUI) "Hidden")
  (bind _returnvalue_2 (Sequencer|Player|CreateLevelSequencePlayer "/Game/EthanBluePrints/LS_AxeHitAnimation.LS_AxeHitAnimation"))
  (Variables|Default|SetAnimation _returnvalue_2))

(event EventTick
  (params (DeltaSeconds :type Float%20%28single-precision%29))
  (bind _out_hit_hit_actor (CallFunction|Raycast (Variables|Default|GetVisibilityDistance)))
  (bind _asbp_destroyable (Utilities|Casting|CastToBP_Destroyable _out_hit_hit_actor)
    (:then
      (Variables|Default|SetCurrentDestroyable _asbp_destroyable)
      (Default|SetVisibilityDamagesOfDestroyable (Variables|Default|GetMyUI) "Visible")
      (Default|GetDamages (Variables|Default|GetCurrentDestroyable))
      (Variables|/Game/EthanBluePrints/BP_Destroyable.BP_Destroyable_C|SetCanHeal (Variables|Default|GetCurrentDestroyable) false))
    (:CastFailed
      (if (Utilities|IsValid (Variables|Default|GetCurrentDestroyable))
        (Variables|/Game/EthanBluePrints/BP_Destroyable.BP_Destroyable_C|SetCanHeal (Variables|Default|GetCurrentDestroyable) true)
        (Variables|Default|SetCurrentDestroyable 0))
      (Default|SetVisibilityDamagesOfDestroyable (Variables|Default|GetMyUI) "Hidden"))))

(event Input|ActionEvents|InputActionAttack
  (params (Key :type Key%20Structure :default "None"))
  (bind _currentdestroyable (Variables|Default|GetCurrentDestroyable))
  (bind _animation (Variables|Default|GetAnimation))
  (:Pressed
    (Variables|Default|SetStayInputAttack true)
    (if (Variables|Default|GetGotAxe) :!label _label
      (if (not (Variables|Default|GetHitInCD))
        (Sequencer|Player|Play _animation :!class /Script/MovieScene.MovieSceneSequencePlayer)
        (Variables|Default|SetHitInCD true)
        (Utilities|FlowControl|Delay 0.4)
        (if (Utilities|IsValid _currentdestroyable)
          (Default|Destroying _currentdestroyable (Variables|Default|GetDamages)))
        (Utilities|FlowControl|Delay (- (Class|TimeManagementBlueprintLibrary|ToSeconds(QualifiedFrameTime) (Class|MovieSceneSequencePlayer|GetEndTime _animation)) 0.4))
        (Variables|Default|SetHitInCD false)
        (if (Variables|Default|GetStayInputAttack)
          (goto _label)))))
  (:Released
    (Variables|Default|SetStayInputAttack false)))

(event Input|ActionEvents|InputActionSpecialAttack
  (params (Key :type Key%20Structure :default "None"))
  (bind _fpc (Variables|Default|GetFPC))
  (bind _axe (Variables|/Game/FirstPersonBP/Blueprints/FirstPersonCharacter.FirstPersonCharacter_C|GetAxe _fpc))
  (bind _returnvalue (Transformation|GetWorldRotation _axe))
  (:Pressed
    (if (Variables|Default|GetGotAxe)
      (bind _out_hit_impact_point (CallFunction|Raycast 1e+09))
      (if (Math|Vector|NotEqual(Vector) _out_hit_impact_point "0, 0, 0" 0.0001)
        (Variables|Default|SetGotAxe false)
        (Rendering|SetVisibility (Variables|/Game/FirstPersonBP/Blueprints/FirstPersonCharacter.FirstPersonCharacter_C|GetAxe (Variables|Default|GetFPC)) false false)
        (bind _returnvalue_2 (Game|SpawnActorfromClass "/Game/EthanBluePrints/BP_AxeProjectile.BP_AxeProjectile_C" (Transformation|GetActorTransform (Variables|Default|GetFPC)) "Undefined" 0 0))
        (bind _output_get (Variables|Default|SetAxeProjectile _returnvalue_2))
        (Transformation|SetActorRelativeLocation _output_get (Transformation|GetWorldLocation _axe))
        (Transformation|SetActorRotation (Variables|Default|GetAxeProjectile) _returnvalue)
        (bind _returnvalue_3 (Game|SpawnActorfromClass "/Game/EthanBluePrints/BP_TargetForAxe.BP_TargetForAxe_C" (Transformation|GetActorTransform (Variables|Default|GetFPC)) "Undefined" 0 0))
        (Transformation|SetActorLocation _returnvalue_3 _out_hit_impact_point false false)
        (Default|SetTargetOfAxe (Variables|Default|GetAxeProjectile) _returnvalue_3)
        (Variables|/Game/EthanBluePrints/BP_AxeProjectile.BP_AxeProjectile_C|SetOriginalRotation (Variables|Default|GetAxeProjectile) _returnvalue)))))

(fn ConstructionScript)

(fn Raycast
  (params (Distance :type Float%20%28single-precision%29))
  (bind _fpc (Variables|Default|GetFPC))
  (bind _firstpersoncamera (Variables|/Game/FirstPersonBP/Blueprints/FirstPersonCharacter.FirstPersonCharacter_C|GetFirstPersonCamera _fpc))
  (bind _returnvalue (Transformation|GetWorldLocation _firstpersoncamera))
  (bind _outhit (Collision|LineTraceByChannel _returnvalue (+ _returnvalue (* (Math|Vector|GetForwardVector _firstpersoncamera) Distance)) "TraceTypeQuery1" false 0 "None"))
  (return (.impactpoint _outhit) (.hitactor _outhit)))