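; BP_PickUp is a pickup actor that reacts when the first-person character touches it.
; On BeginPlay it caches the MC and FPC references from GetMC and GetFPC.
; A Collision sphere, sized from Radius in the construction script, calls PerformAction when its overlapping actor casts to FirstPersonCharacter.
; PerformAction is an empty event here, so this Blueprint defines no pickup effect itself.
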(event OnComponentBeginOverlap(Collision)
  (params (OverlappedComponent :type Primitive%20Component%20Object%20Reference) (OtherActor :type Actor%20Object%20Reference) (OtherComp :type Primitive%20Component%20Object%20Reference) (OtherBodyIndex :type Integer) (bFromSweep :type Boolean) (SweepResult :type Hit%20Result%20Structure%20%28by%20ref%29))
  (Utilities|Casting|CastToFirstPersonCharacter OtherActor)
  (CallFunction|PerformAction))

(event Custom|PerformAction)

(event EventBeginPlay
  (bind _mc (CallFunction|GetMC))
  (Variables|Default|SetMC _mc)
  (bind _fpc (CallFunction|GetFPC))
  (Variables|Default|SetFPC _fpc))

(event Collision|EventActorBeginOverlap
  (params (OtherActor :type Actor%20Object%20Reference)))

(event EventTick
  (params (DeltaSeconds :type Float%20%28single-precision%29)))

(fn ConstructionScript
  (Components|Sphere|SetSphereRadius (Variables|Default|GetCollision) (Variables|Default|GetRadius) true))