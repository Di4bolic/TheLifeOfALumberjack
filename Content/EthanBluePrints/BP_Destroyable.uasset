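; BP_Destroyable is an actor with a configurable mesh that accumulates damage and destroys itself when it reaches DamagesMax.
; Destroying feeds damage into SetDamages, which floors the total at zero and otherwise sends the damage ratio to the MC's UI.
; When CanHeal is set, Tick applies SelfHeal through the same function, with the tick interval set to TimeBeforeHeal as the heal timer.
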(event Custom|Destroying
  (params (Damages :type Float%20%28single-precision%29))
  (CallFunction|SetDamages Damages))

(event Custom|DestroyIt
  (Actor|DestroyActor))

(event EventBeginPlay
  (bind _mc (CallFunction|GetMC))
  (Variables|Default|SetMC _mc)
  (Actor|Tick|SetActorTickInterval (Variables|Default|GetTimeBeforeHeal)))

(event Collision|EventActorBeginOverlap
  (params (OtherActor :type Actor%20Object%20Reference)))

(event EventTick
  (params (DeltaSeconds :type Float%20%28single-precision%29))
  (if (Variables|Default|GetCanHeal)
    (CallFunction|SetDamages (Variables|Default|GetSelfHeal))))

(fn ConstructionScript
  (Components|StaticMesh|SetStaticMesh (Variables|Default|GetStaticMesh) (Variables|Default|GetYourMesh)))

(fn SetDamages
  (params (DamagesValue :type Float%20%28single-precision%29))
  (if (<= (+ (Variables|Default|GetDamages) DamagesValue) 0.0)
    (Variables|Default|SetDamages 0.0)
    (else
      (Variables|Default|SetDamages (+ DamagesValue (Variables|Default|GetDamages)))
      (Default|SetLifeOfDestroyable (Variables|/Game/EthanBluePrints/BP_MyController.BP_MyController_C|GetMyUI (Variables|Default|GetMC)) (/ (Variables|Default|GetDamages) (Variables|Default|GetDamagesMax)))
      (if (>= (Variables|Default|GetDamages) (Variables|Default|GetDamagesMax))
        (CallFunction|DestroyIt)))))

(fn GetDamages
  (Default|SetLifeOfDestroyable (Variables|/Game/EthanBluePrints/BP_MyController.BP_MyController_C|GetMyUI (Variables|Default|GetMC)) (/ (Variables|Default|GetDamages) (Variables|Default|GetDamagesMax))))