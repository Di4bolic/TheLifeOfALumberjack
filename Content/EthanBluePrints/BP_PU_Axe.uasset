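; BP_PU_Axe is an axe pickup that hands the player the axe and starts the wood-cutting objective.
; Its PerformAction event shows the axe on the FPC reference and sets the GotAxe flag on MC.
; It then updates the MC's UI with the quest text and throw and break control hints, and destroys itself.
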(event EventBeginPlay
  (|CallParentFunction) ; This node is disabled and will not be called.\nDrag off pins to build functionality.
)

(event Collision|EventActorBeginOverlap
  (params (OtherActor :type Actor%20Object%20Reference))
  (|CallParentFunction OtherActor) ; This node is disabled and will not be called.\nDrag off pins to build functionality.
)

(event EventTick
  (params (DeltaSeconds :type Float%20%28single-precision%29))
  (|CallParentFunction DeltaSeconds) ; This node is disabled and will not be called.\nDrag off pins to build functionality.
)

(event EventPerformAction
  (Rendering|SetVisibility (Variables|/Game/FirstPersonBP/Blueprints/FirstPersonCharacter.FirstPersonCharacter_C|GetAxe (Variables|Default|GetFPC)) true false)
  (Variables|/Game/EthanBluePrints/BP_MyController.BP_MyController_C|SetGotAxe (Variables|Default|GetMC) true)
  (bind _mc (CallFunction|GetMC))
  (Rendering|Components|TextRender|SetText (Variables|/Game/EthanBluePrints/WBP_PlayerUI.WBP_PlayerUI_C|GetQuest (Variables|/Game/EthanBluePrints/BP_MyController.BP_MyController_C|GetMyUI _mc)) "Go cut wood !")
  (Rendering|Components|TextRender|SetText (Variables|/Game/EthanBluePrints/WBP_PlayerUI.WBP_PlayerUI_C|GetFait1 (Variables|/Game/EthanBluePrints/BP_MyController.BP_MyController_C|GetMyUI _mc)) "Press right click to throw")
  (Widget|SetVisibility (Variables|/Game/EthanBluePrints/WBP_PlayerUI.WBP_PlayerUI_C|GetFait1 (Variables|/Game/EthanBluePrints/BP_MyController.BP_MyController_C|GetMyUI _mc)) "Visible")
  (Rendering|Components|TextRender|SetText (Variables|/Game/EthanBluePrints/WBP_PlayerUI.WBP_PlayerUI_C|GetFait2 (Variables|/Game/EthanBluePrints/BP_MyController.BP_MyController_C|GetMyUI _mc)) "Press left click to break")
  (Widget|SetVisibility (Variables|/Game/EthanBluePrints/WBP_PlayerUI.WBP_PlayerUI_C|GetFait2 (Variables|/Game/EthanBluePrints/BP_MyController.BP_MyController_C|GetMyUI _mc)) "Visible")
  (Actor|DestroyActor))

(fn ConstructionScript
  (|CallParentFunction))