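; BP_Enemy is an enemy actor with hit points and a widget component showing a health bar and name.
; BeginPlay initializes the widget's name and fills the bar, while the construction script places the widget at the PosUI relative location.
; SetLife subtracts damage from HP, sends the HP/HPMax ratio to the widget, and destroys the actor at zero or below.
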(event EventBeginPlay
  (bind _widget (Variables|Default|GetWidget))
  (bind _returnvalue (UserInterface|GetWidget _widget))
  (bind _aswbp__health_bar_and_name (Utilities|Casting|CastToWBP¨_HealthBarAndName _returnvalue))
  (Default|SetName _aswbp__health_bar_and_name)
  (Progress|SetPercent (Variables|/Game/EthanBluePrints/WBP¨_HealthBarAndName.WBP¨_HealthBarAndName_C|GetLife _aswbp__health_bar_and_name) 1.0))

(event Collision|EventActorBeginOverlap
  (params (OtherActor :type Actor%20Object%20Reference)))

(event EventTick
  (params (DeltaSeconds :type Float%20%28single-precision%29)))

(fn ConstructionScript
  (Transformation|SetRelativeLocation (Variables|Default|GetWidget) (Variables|Default|GetPosUI) false false))

(fn SetLife
  (params (Damages :type Float%20%28single-precision%29))
  (Variables|Default|SetHP (- (Variables|Default|GetHP) Damages))
  (Default|SetLife (.AsWBP¨%20Health%20Bar%20and%20Name (Utilities|Casting|CastToWBP¨_HealthBarAndName (UserInterface|GetWidget (Variables|Default|GetWidget)))) (/ (Variables|Default|GetHP) (Variables|Default|GetHPMax)))
  (if (<= (Variables|Default|GetHP) 0.0)
    (Actor|DestroyActor)))