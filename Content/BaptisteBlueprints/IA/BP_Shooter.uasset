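; BP_Shooter is an enemy character Blueprint for a shooter AI that keeps facing the player.
; On BeginPlay it runs BT_ShooterBehavior through AIC_EnemyController, sets up BB_ShooterBoard with the player pawn and records its starting height.
; Each tick it writes DistanceToPlayer to the blackboard and turns toward the player with pitch zeroed.
; It also snaps back to that starting Z whenever its height changes.
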(event EventTick
  (params (DeltaSeconds :type Float%20%28single-precision%29))
  (bind _returnvalue (Game|GetPlayerCharacter 0))
  (bind _returnvalue_2 (Transformation|GetActorLocation))
  (bind _returnvalue_3 (Transformation|GetActorLocation))
  (bind _returnvalue_4 (Transformation|GetActorLocation _returnvalue))
  (bind (_x _y) (Math|Vector|BreakVector _returnvalue_2))
  (bind _returnvalue_5 (Math|Rotator|FindLookatRotation _returnvalue_3 _returnvalue_4))
  (bind (_roll _pitch _yaw) (Math|Rotator|BreakRotator _returnvalue_5))
  (AI|Components|Blackboard|SetValueasFloat (AI|GetBlackboard 0) (Utilities|Name|MakeLiteralName "DistanceToPlayer") (Transformation|GetDistanceTo _returnvalue))
  (Transformation|SetActorRotation (Math|Rotator|MakeRotator _roll 0.0 _yaw))
  (if (not (== (.Z (Math|Vector|BreakVector (Transformation|GetActorLocation self))) (Variables|Default|GetPosZ)))
    (Transformation|SetActorLocation (Math|Vector|MakeVector _x _y (Variables|Default|GetPosZ)) false false)))

(event EventBeginPlay
  (|CallParentFunction)
  (bind _asaic_enemy_controller (Utilities|Casting|CastToAIC_EnemyController (Pawn|GetController)))
  (AI|RunBehaviorTree _asaic_enemy_controller "/Game/BaptisteBlueprints/IA/BT_ShooterBehavior.BT_ShooterBehavior")
  (bind _blackboardcomponent (Class|AIController|UseBlackboard _asaic_enemy_controller "/Game/BaptisteBlueprints/IA/BB_ShooterBoard.BB_ShooterBoard"))
  (AI|Components|Blackboard|SetValueasObject _blackboardcomponent (Utilities|Name|MakeLiteralName "Player") (Game|Player|GetPlayerPawn 0))
  (Variables|Default|SetPosZ (.Z (Math|Vector|BreakVector (Transformation|GetActorLocation self)))))

(fn ConstructionScript
  (|CallParentFunction))